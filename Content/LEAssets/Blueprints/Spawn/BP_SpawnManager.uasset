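; Spawn manager that keeps adding random animals to the level, acting as a simple animal factory.
; On BeginPlay, a looping timer calls SpawnRandom every SpawnInterval seconds.
; Each call picks a random class from Animals and spawns it at a random SpawnPads collider's X/Y, with Z fixed at zero and collisions ignored.
; A sparks emitter node is left unconnected and never runs.
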(event `self.ReceiveBeginPlay`
  ;[1 1 1] From the very start, spawn a random animal every x seconds, x = SpawnInterval (default = 3.0)
  (`KismetSystemLibrary.K2_SetTimer` null "SpawnRandom" (`self.SpawnInterval`) true))

(event `SpawnRandom`
  (bind _spawnpads (`self.SpawnPads`))
  (bind _animals (`self.Animals`))
  (bind _returnvalue (`SceneComponent.K2_GetComponentToWorld` (`/Game/LEAssets/Blueprints/Spawn/BP_SpawnPad.Collider` (`|GetArrayItem` _spawnpads (`KismetMathLibrary.RandomIntegerInRange` 0 (- (`KismetArrayLibrary.Array_Length` _spawnpads) 1))))))
  ;[1 1 1] Animal Factory
  ;;[1 1 1] Instantiate the class, output a product from the factory.
  (`|SpawnActorFromClass` (`|GetArrayItem` _animals (`KismetMathLibrary.RandomIntegerInRange` 0 (- (`KismetArrayLibrary.Array_Length` _animals) 1))) (`KismetMathLibrary.MakeTransform` (`KismetMathLibrary.MakeVector` (.x (.location _returnvalue)) (.y (.location _returnvalue)) 0.0)) "AlwaysSpawn" "OverrideRootScale" null null))

(fn `UserConstructionScript`)